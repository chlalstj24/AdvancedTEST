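; Shotgun weapon Blueprint that extends a parent weapon class with spread-shot hitscan firing and its own sound effect.
; ProcessFiring casts several debug-drawn visibility traces from FirePoint in random directions within a cone, ignoring the owner, and applies damage to each trace's hit actor without checking for a hit.
; PlayEffects plays an explosion cue at the actor, Reload defers to the parent, and BeginPlay triggers one Fire after a short delay.
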(event EventReload
  (|CallParentFunction))

(event EventPlayEffects
  (Audio|PlaySoundatLocation "/Game/StarterContent/Audio/Explosion_Cue.Explosion_Cue" (Transformation|GetActorLocation) "0, 0, 0" 1.0 1.0 0.0 0 0 0 0))

(event EventProcessFiring
  (bind _firepoint (Variables|Default|GetFirePoint))
  (bind _returnvalue (Transformation|GetWorldLocation _firepoint))
  (for _index (range 1 5)
    (bind _outhit (Collision|LineTraceByChannel _returnvalue (+ _returnvalue (* (Math|Random|RandomUnitVectorinConeinDegrees (Math|Vector|GetForwardVector _firepoint) 2e+01) (Variables|Default|GetRange))) "TraceTypeQuery1" false (Utilities|Array|MakeArray (Components|GetOwner)) "ForDuration"))
    (if true
      (Game|Damage|ApplyDamage (.HitActor (Collision|BreakHitResult _outhit)) (Variables|Default|GetDamagePerHit) 0 0))))

(event EventBeginPlay
  (|CallParentFunction)
  (Utilities|FlowControl|Delay 3.0)
  (Class|WeaponBase|Fire))

(fn ConstructionScript)